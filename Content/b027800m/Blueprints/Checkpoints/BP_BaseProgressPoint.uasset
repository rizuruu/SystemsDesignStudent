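; Base checkpoint actor that signals when the player reaches a progress point, then switches itself off.
; Overlap of CollisionArea by player 0's pawn, while PointEnabled is set, runs ProgressEffect without passing the overlapping actor.
; ProgressEffect fires EProgressReached with its OverlappedActor input and itself, then calls DisablePoint to clear PointEnabled so the overlap does not retrigger.
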(event `self.CollisionArea.OnComponentBeginOverlap`
  (params (OverlappedComponent :type "PrimitiveComponent Object Reference") (OtherActor :type "Actor Object Reference") (OtherComp :type "PrimitiveComponent Object Reference") (OtherBodyIndex :type Integer) (bFromSweep :type Boolean) (SweepResult :type "HitResult Structure (by ref)"))
  (if (and (`self.PointEnabled`) (== OtherActor (`GameplayStatics.GetPlayerPawn` 0)))
    (`self.ProgressEffect` null)))

(event `ProgressEffect`
  (params (OverlappedActor :type "Actor Object Reference"))
  (`self.E_ProgressReached` OverlappedActor self)
  (`self.DisablePoint`))

(event `DisablePoint`
  (set `self.PointEnabled` false))

(fn `UserConstructionScript`)