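; Base interactable turret that spawns projectiles on a timer and can be switched on and off.
; If enabled at BeginPlay or on enable, it starts a timer at the fire rate, looping when set to repeat.
; Fire spawns the configured projectile class at the ProjectileOrigin transform.
; Interact toggles the turret, and disabling clears the stored timer handle to stop firing.
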(event `self.ReceiveBeginPlay`
  ;[0 0 0] Initialise
  (if (`self.IsEnabled`)
    (`self.ActivateRepeat`)))

(event `ActivateRepeat`
  ;[0 0 0] Activate Looping Firing Timer
  (bind _returnvalue (`KismetSystemLibrary.K2_SetTimerDelegate` (`|CreateDelegate` :!event `Fire`) (`self.FireRate`) (`self.IsRepeating`)))
  (set `self.LoopFireTimer` _returnvalue))

(event `EnableTurret`
  ;[0 0 0] Enable Turret
  (set `self.IsEnabled` true)
  (`self.ActivateRepeat`))

(event `DisableTurret`
  ;[0 0 0] DisableTurret
  (set `self.IsEnabled` false)
  (`self.StopFiring`))

(event `Fire`
  (bind (_returnvalue_location _returnvalue_rotation _returnvalue_scale) (`KismetMathLibrary.BreakTransform` (`SceneComponent.K2_GetComponentToWorld` (`self.ProjectileOrigin`))))
  ;[0 0 0] Fire
  (`|SpawnActorFromClass` (`self.ProjectileClass`) (`KismetMathLibrary.MakeTransform` _returnvalue_location _returnvalue_rotation _returnvalue_scale) "Undefined" "MultiplyWithRoot" null null))

(event `StopFiring`
  (bind _loopfiretimer (`self.LoopFireTimer`))
  ;[0 0 0] Stop Firing
  (if (`KismetSystemLibrary.K2_IsValidTimerHandle` _loopfiretimer)
    (`KismetSystemLibrary.K2_ClearAndInvalidateTimerHandle` _loopfiretimer)))

(event `Interact`
  (`KismetSystemLibrary.PrintString` "Turret Interacted")
  (if (`self.IsEnabled`)
    (`self.DisableTurret`)
    (else
      (`self.EnableTurret`))))

(fn `UserConstructionScript`)