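; BP_BaseGameMode is a base game mode that handles level transitions on completion or failure.
; On BeginPlay it finds every BP_ProgressManager in the level and binds to each one's level-complete and level-failed events.
; Completion opens the TargetLevel of the first manager found, while failure reloads the current level by name.
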(event `self.ReceiveBeginPlay`
  (`self.SetupManagers`))

(event `SetupManagers`
  (bind _outactors (`GameplayStatics.GetAllActorsOfClass` "/Game/b027800m/Blueprints/Managers/BP_ProgressManager.BP_ProgressManager_C"))
  (bind _output_get (set `self.ProgressManager` _outactors))
  (for _array_element _output_get
    (`/Engine/EditorBlueprintResources/StandardMacros.IsValid` _array_element
      (:`Is Valid`
        (add `/Game/b027800m/Blueprints/Managers/BP_ProgressManager.ELevelComplete` _array_element (`|CreateDelegate` :!event `LevelComplete`))
        (add `/Game/b027800m/Blueprints/Managers/BP_ProgressManager.ELevelFailed` _array_element (`|CreateDelegate` :!event `LevelFailed`))))))

(event `LevelComplete`
  (`KismetSystemLibrary.PrintString` "Game Mode: Level Completed")
  (`GameplayStatics.OpenLevel` (`/Game/b027800m/Blueprints/Managers/BP_ProgressManager.TargetLevel` (`|GetArrayItem` (`self.ProgressManager`)))))

(event `LevelFailed`
  (bind _returnvalue (`GameplayStatics.GetCurrentLevelName` true))
  (`GameplayStatics.OpenLevel` (`KismetStringLibrary.Conv_StringToName` _returnvalue)))

(fn `UserConstructionScript`)