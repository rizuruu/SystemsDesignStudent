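; Utility Blueprint that provides shared helpers for camera shake and pickup effects.
; PlayCameraShake starts a given shake class on player 0's camera manager, provided the class is valid.
; SpawnPickupFX spawns the homing-missile Niagara system at a location and, for a valid target, passes it a trail color and the target's root position.
; That position is sampled once at spawn, so the function does not update it as the target moves.
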(fn `Play Camera Shake`
  (params (`Shake Class` :type "CameraShakeBase Class Reference"))
  (if (`KismetSystemLibrary.IsValidClass` `Shake Class`)
    (`PlayerCameraManager.StartCameraShake` :`self` (`GameplayStatics.GetPlayerCameraManager` null) :`ShakeClass` `Shake Class`)))

(fn `SpawnPickupFX`
  (params (Location :type "Vector Structure") (Target :type "Actor Object Reference") (FXColor :type "LinearColor Structure"))
  (locals (Missiles :type "NiagaraComponent Object Reference"))
  (bind _missiles (`local.Missiles`))
  (bind _returnvalue (`NiagaraFunctionLibrary.SpawnSystemAtLocation` null "/Game/StudentWork/Particles/NS_Homing_Missile.NS_Homing_Missile" Location))
  (set `local.Missiles` _returnvalue)
  (`/Engine/EditorBlueprintResources/StandardMacros.IsValid` Target
    (:`Is Valid`
      (`NiagaraComponent.SetVariableVec3` _missiles "HomingTarget" (`SceneComponent.K2_GetComponentLocation` (`Actor.RootComponent` Target)))
      (`NiagaraComponent.SetVariableLinearColor` _missiles "TrailColor" FXColor))))