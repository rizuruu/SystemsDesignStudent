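; BP_BaseInstance stores the player's health, lives and coin count, apparently as a game instance that keeps them outside the character.
; InitialisePlayerRef caches the player character, and UpdatePlayerInformation copies current health, lives and total coins from that reference without a validity check.
; ResetDefaults restores starting values, setting health and coins to zero and refilling lives.
; The file only saves these values and never writes them back to the character.
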(event `UpdatePlayerInformation`
  (bind _player_character (`self.Player Character`))
  (set `self.Player Health` (`/Game/b027800m/Blueprints/BP_BaseCharacter.Current Health` _player_character))
  (set `self.Player Lives` (`/Game/b027800m/Blueprints/BP_BaseCharacter.PlayerLives` _player_character))
  (set `self.Player Coins` (`/Game/b027800m/Blueprints/BP_BaseCharacter.Total Coins` _player_character)))

(event `InitialisePlayerRef`
  (params (PlayerCharacter :type "/Game/b027800m/Blueprints/BP_BaseCharacter Object Reference"))
  (set `self.Player Character` PlayerCharacter))

(event `ResetDefaults`
  (set `self.Player Health` 0.0)
  (set `self.Player Lives` 3)
  (set `self.Player Coins` 0))