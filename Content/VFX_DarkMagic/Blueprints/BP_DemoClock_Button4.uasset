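; Demo clock actor from the dark magic VFX set, with moving hands, a swinging pendulum and a glow effect toggled by key 4.
; Tick sets hour and minute hands from system time, the second hand from game time, and swings the pendulum by sine deltas.
; Key 4 plays or reverses a timeline driving dynamic material Bias and Intensity, toggling Niagara eye and glow systems.
; A DoOnce, reset shortly after key release, throttles toggling.
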(event `self.ReceiveBeginPlay`
  (bind _materialcontrol (`self.MaterialControl`))
  (bind _hue (`self.Hue`))
  (`self.EnableInput` (`GameplayStatics.GetPlayerController` 0))
  (`self.SettingMateriaClock`)
  (`MaterialInstanceDynamic.SetScalarParameterValue` _materialcontrol "Bias" (`self.Bias`))
  (`MaterialInstanceDynamic.SetScalarParameterValue` _materialcontrol "Intensity" 0.0)
  (`MaterialInstanceDynamic.SetScalarParameterValue` _materialcontrol "Hue" (- 1.0 _hue))
  (`NiagaraComponent.SetNiagaraVariableFloat` (`self.NS_Glow`) "User.HueColor" _hue)
  (`NiagaraComponent.SetNiagaraVariableFloat` (`self.NS_Eye_2`) "User.HueColor" _hue))

(event `self.ReceiveTick`
  (params (DeltaSeconds :type "Float (single-precision)"))
  ;[1 1 1] Clock
  (`self.F_ActorClock` (`self.SM_Hour_02`) (`self.SM_Minute_02`) (`self.SM_Second_02`))
  (`self.F_PendulumForHours` DeltaSeconds (`self.Angle`) (`self.RotateSpeed`) (`self.RunningTime `) (`self.SM_Balance_02`)))

(event `Key|Four`
  (params (Key :type "Key Structure"))
  (bind _materialcontrol (`self.MaterialControl`))
  (:`Pressed`
    (`/Engine/EditorBlueprintResources/StandardMacros.DoOnce` false :!label _label
      (:`Completed`
        (`/Engine/EditorBlueprintResources/StandardMacros.FlipFlop`
          (:`A`
            (set `self.Begin` true)
            (`ActorComponent.Activate` (`self.NS_Eye_2`) true)
            (`ActorComponent.Activate` (`self.NS_Glow`) true)
            (bind (_direction _animate) (`Timeline|Animate` :!label _label_2)
              (:`Update`
                (`MaterialInstanceDynamic.SetScalarParameterValue` _materialcontrol "Bias" (`KismetMathLibrary.Lerp` 0.0 0.6 _animate))
                (`MaterialInstanceDynamic.SetScalarParameterValue` _materialcontrol "Intensity" (`KismetMathLibrary.Lerp` 0.0 3.0 _animate)))))
          (:`B`
            (set `self.Begin` false)
            (`ActorComponent.Deactivate` (`self.NS_Eye_2`))
            (`ActorComponent.Deactivate` (`self.NS_Glow`))
            (goto _label_2 :!via `Reverse`))))))
  (:`Released`
    (`KismetSystemLibrary.Delay` 2.4)
    (goto _label :!via `Reset`)))

(fn `F_ActorClock`
  (params (SM_HourHand :type "StaticMeshComponent Object Reference") (SM_MinuteHand :type "StaticMeshComponent Object Reference") (SM_SecondHand :type "StaticMeshComponent Object Reference"))
  (bind _returnvalue (`KismetMathLibrary.Now`))
  (bind _returnvalue_2 (`KismetMathLibrary.GetMinute` _returnvalue))
  ;[1 1 1] Clock
  ;;[1 1 1] Hour hand
  (`SceneComponent.K2_SetRelativeRotation` SM_HourHand (`KismetMathLibrary.MakeRotator` 0.0 (* (+ (* (+ (* (`KismetMathLibrary.GetHour12` _returnvalue) 60.0) (`KismetMathLibrary.Conv_IntToDouble` _returnvalue_2)) 60.0) (`KismetMathLibrary.Conv_IntToDouble` 0)) 0.008333)) false false)
  ;;[1 1 1] Minute hand
  (`SceneComponent.K2_SetRelativeRotation` SM_MinuteHand (`KismetMathLibrary.MakeRotator` 0.0 (* (+ 0.0 (* _returnvalue_2 60.0)) 0.1)) false false)
  ;;[1 1 1] Second hand
  (`SceneComponent.K2_SetRelativeRotation` SM_SecondHand (`KismetMathLibrary.MakeRotator` 0.0 (* (`KismetMathLibrary.FTrunc` (`KismetSystemLibrary.GetGameTimeInSeconds`)) 6.0)) false false))

(fn `F_PendulumForHours`
  (params (DeltaTime :type "Float (double-precision)") (Anlge :type "Float (double-precision)") (RotateSpeed :type "Float (double-precision)") (RunningTime :type "Float (double-precision)") (SM_Balance :type "StaticMeshComponent Object Reference"))
  ;[1 1 1] Pendulum for hours
  (bind _output_get (set `self.MyDeltaTime` (* DeltaTime RotateSpeed)))
  (bind _output_get_2 (set `self.DeltaHeight ` (- (`KismetMathLibrary.Sin` (+ _output_get (`self.RunningTime `))) (`KismetMathLibrary.Sin` (`self.RunningTime `)))))
  (`SceneComponent.K2_AddLocalRotation` SM_Balance (`KismetMathLibrary.MakeRotator` 0.0 (* _output_get_2 Anlge)) false false)
  (set `self.RunningTime ` (+ RunningTime (`self.MyDeltaTime`))))

(fn `SettingMateriaClock`
  (bind _returnvalue (`PrimitiveComponent.CreateDynamicMaterialInstance` (`self.SM_Base_02`) 0 "/Game/VFX_DarkMagic/MaterialInstans/MI_BaseClock.MI_BaseClock" "None"))
  (set `self.MaterialControl` _returnvalue))

(fn `UserConstructionScript`)