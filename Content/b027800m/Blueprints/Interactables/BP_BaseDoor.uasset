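; Base door interactable that tracks a lock state and holds references to linked keys, with opening behavior left empty.
; InitialiseLinkedKeys binds an event to the key-collected dispatcher of each valid linked key.
; ActivateDoor clears the lock, and any overlap on DoorCollision while unlocked calls OpenDoor.
; OpenDoor and KeyCollected are empty events, so this graph neither moves the door nor reacts to collected keys.
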(event `InitialiseLinkedKeys`
  ;[0 0 0] Initialise All Linked Keys
  (for _array_element (`self.LinkedKeys`)
    (`/Engine/EditorBlueprintResources/StandardMacros.IsValid` _array_element
      (:`Is Valid`
        (add `/Game/b027800m/Blueprints/Pickups/BP_BaseKeyPickup.E_KeyCollected` _array_element (`|CreateDelegate` :!event `KeyCollected`))))))

(event `ActivateDoor`
  (set `self.IsLocked?` false))

(event `self.DoorCollision.OnComponentBeginOverlap`
  (params (OverlappedComponent :type "PrimitiveComponent Object Reference") (OtherActor :type "Actor Object Reference") (OtherComp :type "PrimitiveComponent Object Reference") (OtherBodyIndex :type Integer) (bFromSweep :type Boolean) (SweepResult :type "HitResult Structure (by ref)"))
  (if (not (`self.IsLocked?`))
    (`self.OpenDoor`)))

(event `OpenDoor`)

(event `KeyCollected`)

(fn `UserConstructionScript`)