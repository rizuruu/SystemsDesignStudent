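; Demo actor for the VFX_DarkMagic pack that shows a selected Niagara portal effect with an adjustable hue.
; BeginPlay pushes HueColor into the Niagara component's User.HueColor parameter.
; Tick keeps calling Play on a timeline, whose updates assign NSPortalSelection to that component and activate it without a reset.
; Each update also feeds a four-second Delay that restarts the timeline from the start, forming a repeating loop.
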(event `self.ReceiveBeginPlay`
  (`NiagaraComponent.SetNiagaraVariableFloat` (`self.NS`) "User.HueColor" (`self.Hue_Color`)))

(event `self.ReceiveTick`
  (params (DeltaSeconds :type "Float (single-precision)"))
  (`Timeline|Timeline_0` :!label _label
    (:`Update`
      (`self.Activation_NS`)
      (`KismetSystemLibrary.Delay` 4.0)
      (goto _label :!via `PlayFromStart`))))

(fn `Activation_NS`
  (bind _ns (`self.NS`))
  (`NiagaraComponent.SetAsset` _ns (`self.NS_PortalSelection`))
  (`ActorComponent.SetActive` _ns true false))

(fn `UserConstructionScript`)