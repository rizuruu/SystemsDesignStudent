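; BP_PortalsDemo is a demo actor that shows a selectable Niagara portal effect when something enters its trigger box.
; BeginPlay writes the Hue variable into the effect's User.HueColor parameter.
; Box overlap calls ActivationNS, which assigns NSPortalSelection to the Portals component and activates it without reset.
; Ending the overlap deactivates the component.
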(event `self.ReceiveBeginPlay`
  (`NiagaraComponent.SetNiagaraVariableFloat` (`self.Portals`) "User.HueColor" (`self.Hue`)))

(event `self.Box.OnComponentBeginOverlap`
  (params (OverlappedComponent :type "PrimitiveComponent Object Reference") (OtherActor :type "Actor Object Reference") (OtherComp :type "PrimitiveComponent Object Reference") (OtherBodyIndex :type Integer) (bFromSweep :type Boolean) (SweepResult :type "HitResult Structure (by ref)"))
  (`self.Activation_NS`))

(event `self.Box.OnComponentEndOverlap`
  (params (OverlappedComponent :type "PrimitiveComponent Object Reference") (OtherActor :type "Actor Object Reference") (OtherComp :type "PrimitiveComponent Object Reference") (OtherBodyIndex :type Integer))
  (`ActorComponent.Deactivate` (`self.Portals`)))

(fn `Activation_NS`
  (bind _portals (`self.Portals`))
  (`NiagaraComponent.SetAsset` _portals (`self.NS_PortalSelection`))
  (`ActorComponent.SetActive` _portals true false))

(fn `UserConstructionScript`)