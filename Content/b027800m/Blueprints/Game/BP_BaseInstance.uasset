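; BP_BaseInstance is the game instance that holds player state and game-wide services such as music, pausing and input type.
; It keeps a player character reference and copies health, lives and coins from its PlayerData, with a reset event restoring defaults.
; It plays music as a 2D sound that persists across level transitions.
; Pausing sets game pause, calls the HUD's pause menu toggle and sets mouse cursor visibility.
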(event `UpdatePlayerInformation`
  (bind ((`CurrentHealth_3_3A34AE214CEA6C499CBDB48A851904BB` _currenthealth) (`Coins_8_8F0CC87E447435EDA23D3FA648E2E2C0` _coins) (`Lives_10_332A040147CB58035291058995F3C08B` _lives)) (break `/Game/b027800m/Blueprints/Structs/SPlayerData` (`/Game/b027800m/Blueprints/Game/BP_BaseCharacter.PlayerData` (`self.Player Character`))))
  (set `self.Player Health` _currenthealth)
  (set `self.Player Lives` _lives)
  (set `self.Player Coins` _coins))

(event `InitialisePlayerRef`
  (params (PlayerCharacter :type "/Game/b027800m/Blueprints/Game/BP_BaseCharacter Object Reference"))
  (set `self.Player Character` PlayerCharacter))

(event `ResetDefaults`
  (set `self.Player Health` 0.0)
  (set `self.Player Lives` 3)
  (set `self.Player Coins` 0))

(event `PlayMusic`
  (bind _returnvalue (`GameplayStatics.CreateSound2D` "/Game/b027800m/Audio/The_Wizards_Quest.The_Wizards_Quest" 1.0 1.0 0.0 null true))
  (bind _output_get (set `self.NewVar_0` _returnvalue))
  (`AudioComponent.Play` _output_get 0.0))

(event `SetInputType`
  (params (`IsGamepad?` :type Boolean))
  (set `self.Is Gamepad?` `IsGamepad?`))

(event `PauseGame`
  (params (`Pause?` :type Boolean))
  (`GameplayStatics.SetGamePaused` `Pause?`)
  (`/Game/b027800m/Widgets/Player/WBP_PlayerHUD.TogglePauseMenu` (`/Game/b027800m/Blueprints/Game/BP_BaseCharacter.PlayerHUD` (`self.Player Character`)) false)
  (set `PlayerController.bShowMouseCursor` `Pause?` (`GameplayStatics.GetPlayerController` 0)))

(fn `GetGameInstance`
  (returns (GameInstance :type "/Game/b027800m/Blueprints/Game/BP_BaseInstance Object Reference"))
  (return self))