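; Base Blueprint for interactable objects that shows an interact prompt on the player HUD when an actor comes within range.
; Sphere overlaps check for BPI_PlayerHUD, fetch the HUD widget through it and toggle its interaction message on or off.
; The Interact event only stores the interacting character, and an empty OnEndOverlap event fires on exit as a hook.
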(event `/Game/b027800m/Blueprints/Interfaces/BPI_Interact.Interact`
  (params (`Interacting Character` :type "/Game/b027800m/Blueprints/Game/BP_BaseCharacter Object Reference"))
  (set `self.Interacting Character` `Interacting Character`))

(event `self.Sphere.OnComponentBeginOverlap`
  (params (OverlappedComponent :type "PrimitiveComponent Object Reference") (OtherActor :type "Actor Object Reference") (OtherComp :type "PrimitiveComponent Object Reference") (OtherBodyIndex :type Integer) (bFromSweep :type Boolean) (SweepResult :type "HitResult Structure (by ref)"))
  (if (`KismetSystemLibrary.DoesImplementInterface` OtherActor "/Game/b027800m/Blueprints/Interfaces/BPI_PlayerHUD.BPI_PlayerHUD_C")
    (bind _hud_widget (message `/Game/b027800m/Blueprints/Interfaces/BPI_PlayerHUD.GetHUDWidget` OtherActor))
    (`/Game/b027800m/Widgets/Player/WBP_Interaction.ToggleInteractMessage` (`/Game/b027800m/Widgets/Player/WBP_PlayerHUD.WBP_Interaction` _hud_widget) true)))

(event `self.Sphere.OnComponentEndOverlap`
  (params (OverlappedComponent :type "PrimitiveComponent Object Reference") (OtherActor :type "Actor Object Reference") (OtherComp :type "PrimitiveComponent Object Reference") (OtherBodyIndex :type Integer))
  (if (`KismetSystemLibrary.DoesImplementInterface` OtherActor "/Game/b027800m/Blueprints/Interfaces/BPI_PlayerHUD.BPI_PlayerHUD_C")
    (bind _hud_widget (message `/Game/b027800m/Blueprints/Interfaces/BPI_PlayerHUD.GetHUDWidget` OtherActor))
    (`/Game/b027800m/Widgets/Player/WBP_Interaction.ToggleInteractMessage` (`/Game/b027800m/Widgets/Player/WBP_PlayerHUD.WBP_Interaction` _hud_widget) false)
    (`self.OnEndOverlap`)))

(event `OnEndOverlap`)

(fn `UserConstructionScript`)