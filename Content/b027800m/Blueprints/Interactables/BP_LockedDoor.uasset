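; BP_LockedDoor is an interactable double door that swings open when activated.
; On BeginPlay it initialises its linked keys, and ActivateDoor calls the parent logic before OpenDoor.
; OpenDoor waits briefly for a squeak sound, then plays the Doors timeline, setting both leaves' world rotation through GetDoorRotation.
; The yaw lerp toward zero inside GetDoorRotation is left unconnected.
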(event `self.ReceiveBeginPlay`
  (`self.InitialiseLinkedKeys`))

(event `self.ActivateDoor`
  (`parent.ActivateDoor`)
  (`self.OpenDoor`))

(event `self.OpenDoor`
  ;[0 0 0] Delay for Squeak sound
  (`KismetSystemLibrary.Delay` 0.5)
  (bind (_direction _alpha) (`Timeline|Doors`)
    (:`Update`
      (bind (_door _returnvalue) (`self.GetDoorRotation` (`self.Door_L`) _alpha))
      (`SceneComponent.K2_SetWorldRotation` _door _returnvalue false false)
      (bind (_door_2 _returnvalue_2) (`self.GetDoorRotation` (`self.Door_R`) _alpha))
      (`SceneComponent.K2_SetWorldRotation` _door_2 _returnvalue_2 false false))))

(fn `UserConstructionScript`
  (`parent.UserConstructionScript`))