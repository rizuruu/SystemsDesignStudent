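; BP_ProgressManager tracks level progress, handling checkpoints, level completion, player death and respawning.
; On BeginPlay it binds to each progress point and the player's death event, caches the game instance, and uses the PlayerStart as the initial respawn location.
; Checkpoints move the respawn location to their flag; checkpoints, level end and non-final deaths save through the game instance.
; Running out of lives broadcasts level failure and resets defaults.
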(event `self.ReceiveBeginPlay`
  ;[0 0 0] Begin Play
  (`self.Initialise`)
  (`self.SetupPlayer`)
  (bind _returnvalue (`GameplayStatics.GetActorOfClass` "/Script/Engine.PlayerStart"))
  (set `self.RespawnLocation` (`self.K2_GetActorLocation` _returnvalue))
  (`self.SetupInstance`))

(event `Initialise`
  ;[0 0 0] Initialise
  (for _array_element (`self.ProgressPoints`)
    (`/Engine/EditorBlueprintResources/StandardMacros.IsValid` _array_element
      (:`Is Valid`
        (add `/Game/b027800m/Blueprints/Checkpoints/BP_BaseProgressPoint.E_ProgressReached` _array_element (`|CreateDelegate` :!event `PointReached`))))))

(event `PointReached`
  (params (`Overlapped Actor` :type "Actor Object Reference") (`Progress Point` :type "/Game/b027800m/Blueprints/Checkpoints/BP_BaseProgressPoint Object Reference"))
  ;[0 0 0] Point Reached
  (switch `/Game/b027800m/Blueprints/Enums/E_ProgressPointType` (`/Game/b027800m/Blueprints/Checkpoints/BP_BaseProgressPoint.ProgressType` `Progress Point`)
    (:`NewEnumerator0`
      (`self.CheckpointReached` `Progress Point`))
    (:`NewEnumerator1`
      (`self.LevelEndReached`))))

(event `CheckpointReached`
  (params (Checkpoint :type "/Game/b027800m/Blueprints/Checkpoints/BP_BaseProgressPoint Object Reference"))
  ;[0 0 0] Checkpoint Reached
  (bind _output_get (set `self.RespawnLocation` (`SceneComponent.K2_GetComponentLocation` (`/Game/b027800m/Blueprints/Checkpoints/BP_BaseProgressPoint.FlagMesh` Checkpoint))))
  (`KismetSystemLibrary.PrintString` (`KismetStringLibrary.Concat_StrStr` "Respawn Location: " (`KismetStringLibrary.Conv_VectorToString` _output_get)))
  (`self.SaveData`))

(event `SaveData`
  ;[0 0 0] Save Data
  (`KismetSystemLibrary.PrintString` "Saving Data")
  (`/Game/b027800m/Blueprints/Game/BP_BaseInstance.UpdatePlayerInformation` (`self.GameInstance`)))

(event `LevelEndReached`
  ;[0 0 0] Level End Reached
  (`KismetSystemLibrary.PrintString` "Level End Reached")
  (`self.SaveData`)
  (`self.ELevelComplete`))

(event `SetupPlayer`
  ;[0 0 0] Setup Player
  (bind _asbp_base_character (cast `/Game/b027800m/Blueprints/Game/BP_BaseCharacter` (`GameplayStatics.GetPlayerCharacter` 0)))
  (bind _output_get (set `self.PlayerCharacter` _asbp_base_character))
  (add `/Game/b027800m/Blueprints/Game/BP_BaseCharacter.EPlayerDeath` _output_get (`|CreateDelegate` :!event `PlayerDeath`)))

(event `PlayerDeath`
  (params (LivesRemaining :type Integer))
  ;[0 0 0] Player Death - Respawn or Fail Check
  (`KismetSystemLibrary.PrintString` "Player death")
  (if (<= LivesRemaining 0)
    (`self.ELevelFailed`)
    (`/Game/b027800m/Blueprints/Game/BP_BaseInstance.ResetDefaults` (`self.GameInstance`))
    (else
      (`/Game/b027800m/Blueprints/Game/BP_BaseCharacter.Respawn` (`self.PlayerCharacter`) (`self.RespawnLocation`))
      (`self.SaveData`))))

(event `SetupInstance`
  (bind _asbp_base_instance (cast `/Game/b027800m/Blueprints/Game/BP_BaseInstance` (`GameplayStatics.GetGameInstance`)))
  (set `self.GameInstance` _asbp_base_instance))

(fn `UserConstructionScript`)