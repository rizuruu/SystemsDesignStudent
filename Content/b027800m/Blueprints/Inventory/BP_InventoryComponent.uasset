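; Inventory component that stores picked-up items in a map keyed by inventory type.
; AddItemToInventory stacks the incoming quantity onto any existing entry of that type, or starts a new one, and takes the icon from the incoming item.
; It prints a debug message for the addition, then broadcasts the updated map through the EInventoryUpdated dispatcher.
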(fn `AddItemToInventory`
  (params (InventoryItem :type "/Game/b027800m/Blueprints/Structs/SInventoryItem Structure"))
  (bind (_inventorytype _quantity _icon) (break `/Game/b027800m/Blueprints/Structs/SInventoryItem` InventoryItem))
  (bind (_value _returnvalue) (`BlueprintMapLibrary.Map_Find` (`self.InventoryItems`) _inventorytype))
  (`BlueprintMapLibrary.Map_Add` (`self.InventoryItems`) _inventorytype (make `/Game/b027800m/Blueprints/Structs/SInventoryItem` _inventorytype (`KismetMathLibrary.SelectInt` (+ (`.Quantity_5_5B88A71948D62B8CAD6FE6AD18AE28EC` (break `/Game/b027800m/Blueprints/Structs/SInventoryItem` _value)) _quantity) _quantity _returnvalue) _icon))
  (`KismetSystemLibrary.PrintString` (`KismetStringLibrary.Concat_StrStr` "Added " (`|GetEnumeratorNameAsString` _inventorytype) " to Inventory: " (`KismetStringLibrary.Conv_IntToString` _quantity)) true true (struct :`G` 1.0 :`B` 0.047269 :`A` 1.0))
  (`self.EInventoryUpdated` (`self.InventoryItems`)))