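; BP_LockedDoor is a two-panel door meant to open through linked keys, though the key hookup is unfinished.
; On BeginPlay it loops over LinkedKeys and checks validity, but the node binding each key's collected event is disconnected.
; ActivateDoor calls OpenDoor, which prints a debug message and snaps DoorR and DoorL to the same fixed world yaw without animation.
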(event `self.ReceiveBeginPlay`
  (`self.InitialiseLinkedKeys`))

(event `InitialiseLinkedKeys`
  (for _array_element (`self.LinkedKeys`)
    (`/Engine/EditorBlueprintResources/StandardMacros.IsValid` _array_element)))

(event `self.ActivateDoor`
  (`self.OpenDoor`))

(event `OpenDoor`
  (`KismetSystemLibrary.PrintString` "Open the door")
  (`SceneComponent.K2_SetWorldRotation` (`self.Door_R`) (`KismetMathLibrary.MakeRotator` 0.0 0.0 90.0) false false)
  (`SceneComponent.K2_SetWorldRotation` (`self.Door_L`) (`KismetMathLibrary.MakeRotator` 0.0 0.0 90.0) false false))

(fn `UserConstructionScript`
  (`parent.UserConstructionScript`))